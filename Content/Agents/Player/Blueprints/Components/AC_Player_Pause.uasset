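; Player component on BP_FirstPersonCharacter that toggles the pause menu and sets up input and the base HUD.
; The Pause Game input lazily creates one HUD_Pause widget, then adds or removes it while switching game pause, mouse cursor and input mode.
; On BeginPlay it registers IMC_Default through Enhanced Input and shows HUD_base on any level other than MenuMap.
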(event `InputAction|Pause Game` :paused true
  (params (Key :type "Key Structure"))
  (bind _returnvalue (`GameplayStatics.GetPlayerController` 0))
  (bind _returnvalue_2 (`GameplayStatics.GetPlayerController` 0))
  ;[1 1 1] Pause/Unpause le jeu
  (:`Pressed`
    (`/Engine/EditorBlueprintResources/StandardMacros.IsValid` (`self.PauseRef`) ; Si l'HUD pause n'existe pas
      (:`Is Valid`
        _)
      (:`Is Not Valid`
        (bind _returnvalue_3 (`|CreateWidget` "/Game/Scripts/GUI/Menu/Pause_Menu/HUD_Pause.HUD_Pause_C")) ; On le créé
        (set `self.PauseRef` _returnvalue_3)))
    (if (`GameplayStatics.IsGamePaused`)
      (`Widget.RemoveFromParent` (`self.PauseRef`)) ; Sortir de l'HUD pause
      (`GameplayStatics.SetGamePaused` false) ; Retirer la pause du jeu
      (set `PlayerController.bShowMouseCursor` false _returnvalue) ; Retirer la souris
      (`WidgetBlueprintLibrary.SetInputMode_GameOnly` _returnvalue) ; Activer les contrôles in-game
      (else
        (`UserWidget.AddToViewport` (`self.PauseRef`) 0) ; Ajouter a l'écran
        (`GameplayStatics.SetGamePaused` true) ; Mettre le jeu en pause
        (set `PlayerController.bShowMouseCursor` true _returnvalue_2) ; Afficher la souris
        (`WidgetBlueprintLibrary.SetInputMode_GameAndUIEx` _returnvalue_2 (`self.PauseRef`) "LockInFullscreen" false) ; Activer le contrôle type UI (souris/Menu)
      ))))

(event `self.ReceiveBeginPlay`
  (bind _asbp_first_person_character (cast `/Game/Agents/Player/Blueprints/BP_FirstPersonCharacter` (`self.GetOwner`)))
  (bind _asplayer_controller (cast `PlayerController` (`Pawn.GetController` _asbp_first_person_character))
    (:`then`
      (bind _returnvalue (pcsubsystem `EnhancedInputLocalPlayerSubsystem` _asplayer_controller))
      (`/Engine/EditorBlueprintResources/StandardMacros.IsValid` _returnvalue
        (:`Is Valid`
          (`EnhancedInputSubsystemInterface.AddMappingContext` _returnvalue "/Game/Agents/Player/Input/IMC_Default.IMC_Default" 0 (struct))
          ;[1 1 1] Si on est pas dans le menu -> afficher HP
          (bind _returnvalue_2 (`GameplayStatics.GetCurrentLevelName` true))
          (if (not (`KismetStringLibrary.EqualEqual_StrStr` _returnvalue_2 "MenuMap"))
            (bind _returnvalue_3 (`|CreateWidget` "/Game/Scripts/GUI/HUD/HUD_base.HUD_base_C"))
            (`UserWidget.AddToViewport` _returnvalue_3 0)))))
    (:`CastFailed`
      (`KismetSystemLibrary.PrintString` "FAIL"))))