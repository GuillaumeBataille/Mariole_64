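; Player weapon component that fires projectiles for the first-person character when the shoot input is triggered or ongoing.
; With ammo left, it spawns a player projectile at the first-person camera transform and decrements the ammo count.
; The projectile is initialized with the character's aim vector and the component's range, speed, damage and bounce values.
; The ComputeProjectile function is an empty stub.
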(event `EnhancedInput|/Game/Agents/Player/Input/Actions/IA_Shoot`
  (params (ActionValue :type Boolean) (ElapsedSeconds :type "Float (double-precision)") (TriggeredSeconds :type "Float (double-precision)") (InputAction :type "InputAction Object Reference" :default "/Game/Agents/Player/Input/Actions/IA_Shoot.IA_Shoot"))
  (:`Triggered`
    (bind _asbp_first_person_character (cast `/Game/Agents/Player/Blueprints/BP_FirstPersonCharacter` (`self.GetOwner`) :!label _label))
    (if (> (`self.Ammo_Number`) 0)
      (bind _returnvalue (`|SpawnActorFromClass` "/Game/Agents/Player/Blueprints/BP_Player_Projectile.BP_Player_Projectile_C" (`SceneComponent.K2_GetComponentToWorld` (`/Game/Agents/Player/Blueprints/BP_FirstPersonCharacter.FirstPersonCamera` _asbp_first_person_character)) "AlwaysSpawn" "OverrideRootScale" null false null))
      (bind _returnvalue_2 (`/Game/Agents/Player/Blueprints/BP_FirstPersonCharacter.getAimVector` _asbp_first_person_character))
      (`/Game/Agents/Player/Blueprints/BP_Player_Projectile.init` _returnvalue _returnvalue_2 (`self.bulletRange`) (`self.bulletSpeed`) (`self.damage`) (`self.Bounce`))
      (set `self.Ammo_Number` (- (`self.Ammo_Number`) 1))))
  (:`Ongoing`
    (goto _label)))

(fn `computeProjectile`)