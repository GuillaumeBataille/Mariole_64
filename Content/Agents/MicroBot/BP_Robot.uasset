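; BP_Robot is a MicroBot agent that damages the first-person player on physical contact.
; A hit on its capsule casts the other actor to BP_FirstPersonCharacter and passes negated DamageDealt to GestionVie on the player's ACPlayerHP component.
; A Cooldown flag, cleared after a one-second delay, limits how often repeated hits deal damage.
; The Blueprint contains no movement or AI logic, and its construction script is empty.
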(event `self.CapsuleComponent.OnComponentHit`
  (params (HitComponent :type "PrimitiveComponent Object Reference") (OtherActor :type "Actor Object Reference") (OtherComp :type "PrimitiveComponent Object Reference") (NormalImpulse :type "Vector Structure") (Hit :type "HitResult Structure (by ref)"))
  (bind _asbp_first_person_character (cast `/Game/Agents/Player/Blueprints/BP_FirstPersonCharacter` OtherActor))
  (if (not (`self.Cooldown`))
    (`/Game/Agents/Player/Blueprints/Components/AC_Player_HP.gestionVie` (`/Game/Agents/Player/Blueprints/BP_FirstPersonCharacter.AC_Player_HP` _asbp_first_person_character) (* (`self.DamageDealt`) -1))
    (set `self.Cooldown` true)
    (`KismetSystemLibrary.Delay` 1.0)
    (set `self.Cooldown` false)))

(fn `UserConstructionScript`)