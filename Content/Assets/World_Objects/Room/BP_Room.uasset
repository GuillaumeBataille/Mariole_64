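; BP_Room is a procedurally generated room actor built from floor and wall tiles.
; Its construction script always randomizes both tile counts, then fills a floor grid and wall rows using instanced mesh components in local space.
; Each of the two wall functions adds two rows, the second offset along Z by the room's size.
; Overlap events only print debug text, and the custom handler binds only within itself.
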(event `self.ReceiveActorBeginOverlap`
  (params (OtherActor :type "Actor Object Reference"))
  (`KismetSystemLibrary.PrintString` (`KismetSystemLibrary.GetDisplayName` OtherActor)))

(event `OnActorBeginOverlap_Event` :!signature `self.OnActorBeginOverlap`
  (params (OverlappedActor :type "Actor Object Reference") (OtherActor :type "Actor Object Reference"))
  (add `self.OnActorBeginOverlap` (delegate `OnActorBeginOverlap_Event`))
  (cast `/Game/Assets/World_Objects/Room/BP_Room` OverlappedActor)
  (`KismetSystemLibrary.PrintString` "Hello"))

(fn `GenerateFloor`
  (for _index (range (`self.NbrTile_Y`))
    (for _index_2 (range (`self.NbrTile_X`))
      (`InstancedStaticMeshComponent.AddInstance` (`self.Floor`) (`KismetMathLibrary.Conv_VectorToTransform` (`KismetMathLibrary.MakeVector` (* _index_2 (`self.TileSize_X`)) (* _index (`self.TileSize_Y`)))) false))))

(fn `GenerateFrontWall`
  (bind _tilesize_x (`self.TileSize_X`))
  (for _index (range (`self.NbrTile_Y`))
    (bind _returnvalue (* (`self.TileSize_Y`) _index))
    (`InstancedStaticMeshComponent.AddInstance` (`self.Wall0`) (`KismetMathLibrary.Conv_VectorToTransform` (`KismetMathLibrary.MakeVector` 0.0 _returnvalue)) false)
    (`InstancedStaticMeshComponent.AddInstance` (`self.Wall0`) (`KismetMathLibrary.Conv_VectorToTransform` (`KismetMathLibrary.MakeVector` 0.0 _returnvalue (+ (* _tilesize_x (`self.NbrTile_X`)) _tilesize_x 100.0))) false)))

(fn `GenerateLeftWall`
  (bind _tilesize_y (`self.TileSize_Y`))
  (for _index (range (`self.NbrTile_X`))
    (bind _returnvalue (* (`self.TileSize_X`) _index -1.0))
    (`InstancedStaticMeshComponent.AddInstance` (`self.Wall3`) (`KismetMathLibrary.Conv_VectorToTransform` (`KismetMathLibrary.GreaterGreater_VectorRotator` (`KismetMathLibrary.MakeVector` _returnvalue) (struct :`Yaw` 90.0))) false)
    (`InstancedStaticMeshComponent.AddInstance` (`self.Wall3`) (`KismetMathLibrary.Conv_VectorToTransform` (`KismetMathLibrary.MakeVector` 0.0 _returnvalue (+ (* (`self.NbrTile_Y`) _tilesize_y) _tilesize_y 100.0))) false)))

(fn `GenerateRoom`
  (`self.GenerateFloor`)
  (`self.GenerateFrontWall`)
  (`self.GenerateLeftWall`))

(fn `RandomizeRoom`
  (bind _returnvalue (`KismetMathLibrary.RandomIntegerInRange` 3 8))
  (set `self.NbrTile_X` _returnvalue)
  (set `self.NbrTile_Y` _returnvalue))

(fn `UserConstructionScript`
  (if true
    (`self.RandomizeRoom`))
  (`self.GenerateRoom`))